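; A carryable item that spends the player's mana to spawn a decoy.
; Pickup attaches it to the given mesh's item socket and disables collision, while Drop detaches it at a target location and restores collision.
; Primary use spawns BP_Decoy at player 0's transform if mana suffices and no valid decoy exists.
; Secondary use calls Deploy on the stored decoy without a validity check.
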(event EventPickup
  (params (skeletalMesh :type Skeletal%20Mesh%20Component%20Object%20Reference))
  (Audio|PlaySound2D "/Game/Audio/SFX/Item_Pickup_Cue.Item_Pickup_Cue" 1.0 1.0 0.0 0 0)
  (Transformation|AttachComponentToComponent skeletalMesh "BPI_ItemSocket" "SnapToTarget" "SnapToTarget" "KeepRelative" true)
  (Collision|SetCollisionEnabled (Variables|Default|GetCollision) "NoCollision")
  (Development|PrintString "PicAttempted"))

(event EventDrop
  (params (targetLocation :type Vector :default "0, 0, 0"))
  (Audio|PlaySound2D "/Game/Audio/Concrete2Steps/concrete2_step_Cue.concrete2_step_Cue" 1.0 1.0 0.0 0 0)
  (Transformation|DetachFromActor "KeepRelative" "KeepRelative" "KeepRelative")
  (Transformation|SetActorLocation targetLocation false false)
  (Collision|SetCollisionEnabled (Variables|Default|GetCollision) "QueryAndPhysics"))

(event EventUsePrimary
  (bind _returnvalue (Game|GetPlayerCharacter 0))
  (bind _asbp_third_person_character (Utilities|Casting|CastToBP_ThirdPersonCharacter _returnvalue))
  (if (>= (Variables|/Game/ThirdPerson/Blueprints/BP_ThirdPersonCharacter.BP_ThirdPersonCharacter_C|GetMana _asbp_third_person_character) 0.3)
    (Utilities|IsValid (Variables|Default|GetDecoy)
      (:Is%20Valid
        (Development|PrintString "Decoy already deployed"))
      (:Is%20Not%20Valid
        (Variables|/Game/ThirdPerson/Blueprints/BP_ThirdPersonCharacter.BP_ThirdPersonCharacter_C|SetMana _asbp_third_person_character (- (Variables|/Game/ThirdPerson/Blueprints/BP_ThirdPersonCharacter.BP_ThirdPersonCharacter_C|GetMana _asbp_third_person_character) 0.3))
        (bind _returnvalue_2 (Game|SpawnActorfromClass "/Game/AI_Blueprints/BP_Decoy.BP_Decoy_C" (Transformation|GetActorTransform _returnvalue) "Undefined" "MultiplyWithRoot" 0 0))
        (Variables|Default|SetDecoy _returnvalue_2)
        (Audio|PlaySound2D "/Game/Audio/SFX/Decoy_Cue.Decoy_Cue" 1.0 1.0 0.0 0 0)))
    (else
      (Development|PrintString "Insufficient Mana"))))

(event EventUseSecondary
  (Default|Deploy (Variables|Default|GetDecoy)))

(fn ConstructionScript)