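; Blood magic item that the player can pick up, drop and use to spend health on spell effects.
; Pickup snaps it to a skeletal mesh socket and disables collision, while drop detaches it at a target location and re-enables collision.
; Primary use converts a random small amount of player health into equal mana.
; Secondary use costs a fixed chunk of health, if enough remains, to halve every BP_EnemyBase's current and maximum health.
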(event EventPickup
  (params (skeletalMesh :type Skeletal%20Mesh%20Component%20Object%20Reference))
  (Transformation|AttachComponentToComponent skeletalMesh "BPI_ItemSocket" "SnapToTarget" "SnapToTarget" "KeepRelative" true)
  (Collision|SetCollisionEnabled (Variables|Default|GetCollision) "NoCollision")
  (Development|PrintString "PicAttempted"))

(event EventDrop
  (params (targetLocation :type Vector :default "0, 0, 0"))
  (Transformation|DetachFromActor "KeepRelative" "KeepRelative" "KeepRelative")
  (Transformation|SetActorLocation targetLocation false false)
  (Collision|SetCollisionEnabled (Variables|Default|GetCollision) "QueryAndPhysics"))

(event EventUsePrimary
  (bind _asbp_third_person_character (Utilities|Casting|CastToBP_ThirdPersonCharacter (Game|GetPlayerCharacter 0)))
  (bind _output_get (Variables|Default|SetCurseStrength (Math|Random|RandomFloatinRange 0.01 0.5)))
  (Default|ChangeHealth _asbp_third_person_character (* _output_get -1.0))
  (Default|ChangeMana _asbp_third_person_character _output_get))

(event EventUseSecondary
  (bind _asbp_third_person_character (Utilities|Casting|CastToBP_ThirdPersonCharacter (Game|GetPlayerCharacter 0)))
  (if (> (Variables|/Game/ThirdPerson/Blueprints/BP_ThirdPersonCharacter.BP_ThirdPersonCharacter_C|GetHealth _asbp_third_person_character) 0.5)
    (Variables|/Game/ThirdPerson/Blueprints/BP_ThirdPersonCharacter.BP_ThirdPersonCharacter_C|SetHealth _asbp_third_person_character (- (Variables|/Game/ThirdPerson/Blueprints/BP_ThirdPersonCharacter.BP_ThirdPersonCharacter_C|GetHealth _asbp_third_person_character) 0.5))
    (bind _outactors (Actor|GetAllActorsOfClass "/Game/AI_Blueprints/BP_EnemyBase.BP_EnemyBase_C"))
    (for _array_element _outactors
      (Variables|/Game/AI_Blueprints/BP_EnemyBase.BP_EnemyBase_C|SetHealth _array_element (* (Variables|/Game/AI_Blueprints/BP_EnemyBase.BP_EnemyBase_C|GetHealth _array_element) 0.5))
      (Variables|/Game/AI_Blueprints/BP_EnemyBase.BP_EnemyBase_C|SetMaxHealth _array_element (* (Variables|/Game/AI_Blueprints/BP_EnemyBase.BP_EnemyBase_C|GetMaxHealth _array_element) 0.5)))
    (else
      (Development|PrintString "Insufficient Health"))))

(fn ConstructionScript)