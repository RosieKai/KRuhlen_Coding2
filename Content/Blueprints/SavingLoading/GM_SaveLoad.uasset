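; Game mode that handles saving and loading of player stats and level state in two separate save slots.
; On BeginPlay it loads each slot or creates a new save object, restoring character stats and a held item looked up by class.
; Level restore calls LoadStateMessage on every saved actor; older coin and door restore logic is left disconnected.
; Save events write the cached objects to their slots and print the result.
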(event Custom|Load%20Player%20Stats
  (bind _player_save (Variables|Default|GetPlayer_Save))
  (bind _returnvalue (SaveGame|DoesSaveGameExist _player_save))
  (if _returnvalue
    (bind _returnvalue_2 (SaveGame|LoadGamefromSlot _player_save))
    (bind _assg_player_stats (Utilities|Casting|CastToSG_PlayerStats _returnvalue_2))
    (Variables|Default|SetSG_PlayerStats _assg_player_stats)
    (bind _asbp_third_person_character (Utilities|Casting|CastToBP_ThirdPersonCharacter (Game|GetPlayerCharacter 0)))
    (Variables|/Game/ThirdPerson/Blueprints/BP_ThirdPersonCharacter.BP_ThirdPersonCharacter_C|SetStamina _asbp_third_person_character (Variables|/Game/Blueprints/SavingLoading/SG_PlayerStats.SG_PlayerStats_C|GetStamina (Variables|Default|GetSG_PlayerStats)))
    (Variables|/Game/ThirdPerson/Blueprints/BP_ThirdPersonCharacter.BP_ThirdPersonCharacter_C|SetHealth _asbp_third_person_character (Variables|/Game/Blueprints/SavingLoading/SG_PlayerStats.SG_PlayerStats_C|GetHealth (Variables|Default|GetSG_PlayerStats)))
    (Variables|/Game/ThirdPerson/Blueprints/BP_ThirdPersonCharacter.BP_ThirdPersonCharacter_C|SetMana _asbp_third_person_character (Variables|/Game/Blueprints/SavingLoading/SG_PlayerStats.SG_PlayerStats_C|GetMana (Variables|Default|GetSG_PlayerStats)))
    (bind _returnvalue_3 (Actor|GetActorOfClass (Utilities|GetClass (Variables|/Game/Blueprints/SavingLoading/SG_PlayerStats.SG_PlayerStats_C|GetheldItem (Variables|Default|GetSG_PlayerStats)))))
    (Default|LoadHeldItem _asbp_third_person_character _returnvalue_3)
    (else
      (bind _returnvalue_4 (SaveGame|CreateSaveGameObject "/Game/Blueprints/SavingLoading/SG_PlayerStats.SG_PlayerStats_C"))
      (Variables|Default|SetSG_PlayerStats _returnvalue_4))))

(event Custom|Save%20Player%20Stats
  (bind _returnvalue (SaveGame|SaveGametoSlot (Variables|Default|GetSG_PlayerStats) (Variables|Default|GetPlayer_Save)))
  (if _returnvalue
    (Development|PrintString "Player Stats Saved Successfully" true true "(R=0.177605,G=0.140878,B=1.000000,A=1.000000)" 5.0)
    (else
      (Development|PrintString "Error: Cannot Save Player Stats" true true "(R=1.000000,G=0.000000,B=0.073312,A=1.000000)" 5.0))))

(event Custom|Load%20Level%20State
  (bind _level_save (Variables|Default|GetLevel_Save))
  (bind _returnvalue (SaveGame|DoesSaveGameExist _level_save))
  (if _returnvalue
    (bind _returnvalue_2 (SaveGame|LoadGamefromSlot _level_save))
    (bind _assg_level_state (Utilities|Casting|CastToSG_LevelState _returnvalue_2))
    (Variables|Default|SetSG_LevelState _assg_level_state)
    (for _array_element (Variables|/Game/Blueprints/SavingLoading/SG_LevelState.SG_LevelState_C|GetsavedActors (Variables|Default|GetSG_LevelState))
      (Class|BPILevelActorSaveable|LoadState(Message) _array_element))
    (else
      (bind _returnvalue_3 (SaveGame|CreateSaveGameObject "/Game/Blueprints/SavingLoading/SG_LevelState.SG_LevelState_C"))
      (Variables|Default|SetSG_LevelState _returnvalue_3))))

(event Custom|Save%20level%20State
  (bind _returnvalue (SaveGame|SaveGametoSlot (Variables|Default|GetSG_LevelState) (Variables|Default|GetLevel_Save)))
  (if _returnvalue
    (Development|PrintString "Level Saved Successfully" true true "(R=0.177605,G=0.140878,B=1.000000,A=1.000000)" 5.0)
    (else
      (Development|PrintString "Error: Cannot Save Level" true true "(R=1.000000,G=0.000000,B=0.073312,A=1.000000)" 5.0))))

(event EventBeginPlay
  (Development|PrintString "Loading Save Load Game Mode" true true "(R=0.610417,G=0.552836,B=0.039423,A=1.000000)" 1e+01)
  (CallFunction|LoadPlayerStats)
  (CallFunction|LoadLevelState))

(fn ConstructionScript)