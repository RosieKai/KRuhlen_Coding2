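; Manager that populates the level with enemies and tops them up when their numbers run low.
; On BeginPlay it visits every BP_EnemySpawnPoint and, on a coin flip, spawns a random class from ActorClass there.
; A self-repeating delayed check counts actors tagged "Enemy", runs another spawn pass below a threshold, and prints debug counts.
; An unconnected chain for randomising enemy name, materials and mesh never runs.
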(event Custom|SpawnEnemies
  (bind _outactors (Actor|GetAllActorsOfClass "/Game/Blueprints/BP_EnemySpawnPoint.BP_EnemySpawnPoint_C"))
  (Development|PrintText (Utilities|Text|FormatText "There are {count} spawn points in the level" (Utilities|Array|Length _outactors)))
  (for _array_element _outactors
    (if (Math|Random|RandomBoolwithWeight 0.5)
      (bind _output_get (Variables|Default|SetSpawnableEnemy (.OutItem (Utilities|Array|Random (Variables|Default|GetActor%20Class)))))
      (bind _returnvalue (Game|SpawnActorfromClass _output_get (Transformation|GetActorTransform _array_element) "Undefined" "MultiplyWithRoot" _array_element 0))
      (Development|PrintText (Utilities|Text|FormatText "Enemy Spawned: {type}" _returnvalue)))))

(event Custom|CheckCount
  (Utilities|FlowControl|Delay 3e+01)
  (bind _outactors (Actor|GetAllActorswithTag "Enemy"))
  (if (< (Utilities|Array|Length _outactors) 15)
    (CallFunction|SpawnEnemies)
    (Development|PrintText (Utilities|Text|FormatText "There WERE {num} Enemies left" (Utilities|Array|Length _outactors)) true true "(R=1.000000,G=0.237792,B=0.000000,A=1.000000)" 5.0)
    (else
      (Development|PrintText (Utilities|Text|FormatText "There are {num} enemies left" (Utilities|Array|Length _outactors)) true true "(R=0.650981,G=1.000000,B=0.134564,A=1.000000)" 5.0)))
  (CallFunction|CheckCount))

(event EventBeginPlay
  (CallFunction|SpawnEnemies)
  (CallFunction|CheckCount))

(fn ConstructionScript)