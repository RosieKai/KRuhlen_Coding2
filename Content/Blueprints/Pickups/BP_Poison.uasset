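; BP_Poison is a pickup that alters the third-person character's mana and health when touched.
; On overlap with the character, it applies its ManaAmount and HealthAmount through the character's change functions, plays a poison sound and destroys itself.
; An untouched pickup also destroys itself after a random delay of roughly 10 to 20 seconds from BeginPlay.
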(event OnComponentBeginOverlap(collision)
  (params (OverlappedComponent :type Primitive%20Component%20Object%20Reference) (OtherActor :type Actor%20Object%20Reference) (OtherComp :type Primitive%20Component%20Object%20Reference) (OtherBodyIndex :type Integer) (bFromSweep :type Boolean) (SweepResult :type Hit%20Result%20Structure%20%28by%20ref%29))
  (bind _asbp_third_person_character (Utilities|Casting|CastToBP_ThirdPersonCharacter OtherActor))
  (Default|ChangeMana _asbp_third_person_character (Variables|Default|GetManaAmount))
  (Default|ChangeHealth _asbp_third_person_character (Variables|Default|GetHealthAmount))
  (Audio|PlaySoundatLocation "/Game/Audio/SFX/PoisonSound_Cue.PoisonSound_Cue" (Transformation|GetActorLocation) "0, 0, 0" 1.0 1.0 0.0 0 0 0 0)
  (Actor|DestroyActor))

(event EventBeginPlay
  (Utilities|FlowControl|Delay (Math|Random|RandomFloatinRange 1e+01 2e+01))
  (Actor|DestroyActor))

(fn ConstructionScript)