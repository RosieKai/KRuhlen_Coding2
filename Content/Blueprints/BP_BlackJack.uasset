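; Holdable item actor that plays a simplified blackjack game, with results shown as printed messages.
; Pickup snaps it to a skeletal mesh socket and disables box collision; Drop places it and resets the game.
; Primary use hits with a random card value, updating the CardCount text and resetting on a bust.
; Secondary use holds, comparing against a randomly rolled dealer total and resetting except on a draw.
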(event EventPickup
  (params (skeletalMesh :type Skeletal%20Mesh%20Component%20Object%20Reference))
  (Development|PrintString "Attempting Card Pick Up")
  (Transformation|AttachComponentToComponent skeletalMesh "BPI_ItemSocket" "SnapToTarget" "SnapToTarget" "KeepRelative" true)
  (Collision|SetCollisionEnabled (Variables|Default|GetBox) "NoCollision")
  (Development|PrintString "PicAttempted"))

(event EventDrop
  (params (targetLocation :type Vector :default "0, 0, 0"))
  (Transformation|DetachFromActor "KeepRelative" "KeepRelative" "KeepRelative")
  (Transformation|SetActorLocation targetLocation false false)
  (Collision|SetCollisionEnabled (Variables|Default|GetBox) "QueryAndPhysics")
  (Variables|Default|SetcardNumbers 0)
  (Variables|Default|SetdealerHand 0)
  (Variables|Default|SetrandInt 0))

(event EventUsePrimary
  (Development|PrintString "\"Hit\"")
  (bind _output_get (Variables|Default|SetrandInt (Math|Random|RandomIntegerinRange 1 13)))
  (bind _output_get_2 (Variables|Default|SetcardNumbers (+ _output_get (Variables|Default|GetcardNumbers))))
  (if (<= _output_get_2 21)
    (Development|PrintText (Utilities|Text|FormatText "You drew a {number}. Your current score is {totalNumber}. 
Hit or Hold?" _output_get _output_get_2) true true "(R=0.000000,G=0.660000,B=1.000000,A=1.000000)" 4.0)
    (Rendering|Components|TextRender|SetText (Variables|Default|GetcardCount) (Utilities|Text|ToText(Integer) _output_get_2))
    (else
      (Development|PrintText (Utilities|Text|FormatText "Tough Luck. You drew a {number} which pushed your score to {totalNumber}. That's a bust." _output_get _output_get_2) true true "(R=0.000000,G=0.660000,B=1.000000,A=1.000000)" 4.0)
      (Variables|Default|SetcardNumbers 0)
      (Rendering|Components|TextRender|SetText (Variables|Default|GetcardCount) (Utilities|Text|ToText(Integer) _output_get_2)))))

(event EventUseSecondary
  (bind _output_get (Variables|Default|SetdealerHand (Math|Random|RandomIntegerinRange 14 23)))
  (Development|PrintText (Utilities|Text|FormatText "Dealer's hand: {dealer} 
Your hand: {You}" _output_get (Variables|Default|GetcardNumbers)) true true "(R=0.000000,G=0.660000,B=1.000000,A=1.000000)" 4.0)
  (if (> (Variables|Default|GetdealerHand) 21)
    (Development|PrintString "The dealer busts! You win!")
    (Variables|Default|SetcardNumbers 0 :!label _label)
    (Variables|Default|SetdealerHand 0)
    (Variables|Default|SetrandInt 0)
    (elif (> (Variables|Default|GetcardNumbers) (Variables|Default|GetdealerHand))
      (Development|PrintString "Your hand is greater! You win!")
      (goto _label)
      (elif (== (Variables|Default|GetcardNumbers) (Variables|Default|GetdealerHand))
        (Development|PrintString "It's a draw!")
        (else
          (Development|PrintString "The dealer's hand is greater. Better luck next time.")
          (goto _label))))))

(event EventBeginPlay
  (Variables|Default|SetcardNumbers 0)
  (Variables|Default|SetrandInt 0))

(fn ConstructionScript)