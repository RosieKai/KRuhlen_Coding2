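; Lightning Rod is a holdable item that spends the player's mana to cast area lightning attacks.
; Pickup attaches it to a socket on the given skeletal mesh and disables collision; drop detaches it at a target location and restores collision.
; Primary use strikes ahead of the player, while costlier secondary use strikes essentially at the player's position, each spawning BP_LightningEffect and applying radial falloff damage.
; Primary's mana check is lower than its actual cost.
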(event EventPickup
  (params (skeletalMesh :type Skeletal%20Mesh%20Component%20Object%20Reference))
  (Audio|PlaySound2D "/Game/Audio/SFX/Item_Pickup_Cue.Item_Pickup_Cue" 1.0 1.0 0.0 0 0)
  (Transformation|AttachComponentToComponent skeletalMesh "BPI_ItemSocket" "SnapToTarget" "SnapToTarget" "KeepRelative" true)
  (Collision|SetCollisionEnabled (Variables|Default|GetCollision) "NoCollision")
  (Development|PrintString "PicAttempted"))

(event EventDrop
  (params (targetLocation :type Vector :default "0, 0, 0"))
  (Audio|PlaySound2D "/Game/Audio/Concrete2Steps/concrete2_step_Cue.concrete2_step_Cue" 1.0 1.0 0.0 0 0)
  (Transformation|DetachFromActor "KeepRelative" "KeepRelative" "KeepRelative")
  (Transformation|SetActorLocation targetLocation false false)
  (Collision|SetCollisionEnabled (Variables|Default|GetCollision) "QueryAndPhysics"))

(event EventUsePrimary
  (bind _returnvalue (Game|GetPlayerCharacter 0))
  (bind _returnvalue_2 (Transformation|GetActorForwardVector _returnvalue))
  (bind _rootcomponent (Variables|/Script/Engine.Actor|GetRootComponent _returnvalue))
  (bind _returnvalue_3 (Transformation|GetWorldLocation _rootcomponent))
  (bind _returnvalue_4 (* _returnvalue_2 "1000.000000,1000.000000,1000.000000"))
  (bind _returnvalue_5 (+ _returnvalue_3 _returnvalue_4))
  (bind _asbp_third_person_character (Utilities|Casting|CastToBP_ThirdPersonCharacter _returnvalue))
  (if (>= (Variables|/Game/ThirdPerson/Blueprints/BP_ThirdPersonCharacter.BP_ThirdPersonCharacter_C|GetMana _asbp_third_person_character) 0.1)
    (Default|ChangeMana _asbp_third_person_character -0.25)
    (Game|SpawnActorfromClass "/Game/Blueprints/BP_LightningEffect.BP_LightningEffect_C" (Math|Transform|MakeTransform _returnvalue_5 "0, 0, 0" "1.000000,1.000000,1.000000") "Undefined" "MultiplyWithRoot" 0 0)
    (Class|GameplayStatics|ApplyRadialDamagewithFalloff 1.5 0.1 _returnvalue_5 1.5e+02 3e+02 2.0 0 0 self 0 "ECC_Visibility")
    (else
      (Development|PrintString "Insufficient Mana"))))

(event EventUseSecondary
  (bind _returnvalue (Game|GetPlayerCharacter 0))
  (bind _returnvalue_2 (Transformation|GetActorForwardVector _returnvalue))
  (bind _rootcomponent (Variables|/Script/Engine.Actor|GetRootComponent _returnvalue))
  (bind _returnvalue_3 (Transformation|GetWorldLocation _rootcomponent))
  (bind _returnvalue_4 (+ _returnvalue_3 _returnvalue_2))
  (bind _asbp_third_person_character (Utilities|Casting|CastToBP_ThirdPersonCharacter _returnvalue))
  (if (>= (Variables|/Game/ThirdPerson/Blueprints/BP_ThirdPersonCharacter.BP_ThirdPersonCharacter_C|GetMana _asbp_third_person_character) 0.75)
    (Default|ChangeMana _asbp_third_person_character -0.75)
    (Game|SpawnActorfromClass "/Game/Blueprints/BP_LightningEffect.BP_LightningEffect_C" (Math|Transform|MakeTransform _returnvalue_4 "0, 0, 0" "1.000000,1.000000,1.000000") "Undefined" "MultiplyWithRoot" 0 0)
    (Class|GameplayStatics|ApplyRadialDamagewithFalloff 2.0 0.5 _returnvalue_4 1.5e+02 3e+02 2.0 0 0 self 0 "ECC_Visibility")
    (else
      (Development|PrintString "Insufficient Mana"))))

(fn ConstructionScript)