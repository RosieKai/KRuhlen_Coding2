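; BP_ItemSpawner is an actor that spawns a random item and replaces it once that item leaves.
; On BeginPlay it picks a random class from Spawnable, spawns it at its root transform and stores it as SpawnedActor.
; When that tracked actor ends overlap with the spawner, it waits DelayDuration and loops back to the same spawn step.
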(event EventBeginPlay
  (bind _returnvalue (Game|SpawnActorfromClass (.OutItem (Utilities|Array|Random (Variables|Default|GetSpawnable))) (Transformation|GetWorldTransform (Variables|Default|GetDefaultSceneRoot)) "Undefined" "MultiplyWithRoot" 0 0))
  (Variables|Default|SetSpawnedActor _returnvalue))

(event Collision|EventActorEndOverlap
  (params (OtherActor :type Actor%20Object%20Reference))
  (if (== OtherActor (Variables|Default|GetSpawnedActor))
    (Utilities|FlowControl|Delay (Variables|SpawnVariables|GetDelay%20Duration))
    (bind _returnvalue (Game|SpawnActorfromClass (.OutItem (Utilities|Array|Random (Variables|Default|GetSpawnable))) (Transformation|GetWorldTransform (Variables|Default|GetDefaultSceneRoot)) "Undefined" "MultiplyWithRoot" 0 0))
    (Variables|Default|SetSpawnedActor _returnvalue)))

(fn ConstructionScript)