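; BP_ElementalBarrier is a barrier that opens for a player character of the matching elemental type.
; On BeginPlay it labels its text render with its type name, such as "Cherry Barrier".
; When a BP_ThirdPersonCharacter overlaps the Collision component, a matching type turns off the Barrier's collision, with no logic here to restore it.
; A mismatch only prints the character's type.
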(event OnComponentBeginOverlap(Collision)
  (params (OverlappedComponent :type Primitive%20Component%20Object%20Reference) (OtherActor :type Actor%20Object%20Reference) (OtherComp :type Primitive%20Component%20Object%20Reference) (OtherBodyIndex :type Integer) (bFromSweep :type Boolean) (SweepResult :type Hit%20Result%20Structure%20%28by%20ref%29))
  (bind _asbp_third_person_character (Utilities|Casting|CastToBP_ThirdPersonCharacter OtherActor))
  (if (Utilities|Enum|Equal(Enum) (Variables|/Game/ThirdPerson/Blueprints/BP_ThirdPersonCharacter.BP_ThirdPersonCharacter_C|GetelementalType _asbp_third_person_character) (Variables|Default|GetelementalTypeBarrier))
    (Collision|SetCollisionEnabled (Variables|Default|GetBarrier) "NoCollision")
    (else
      (Development|PrintString (Utilities|String|EnumtoString (Variables|/Game/ThirdPerson/Blueprints/BP_ThirdPersonCharacter.BP_ThirdPersonCharacter_C|GetelementalType _asbp_third_person_character))))))

(event EventBeginPlay
  (Rendering|Components|TextRender|SetText (Variables|Default|GetTextRender) (Utilities|Text|FormatText "{Type} Barrier" (Utilities|Select :Index (Variables|Default|GetelementalTypeBarrier) :NewEnumerator0 "Mundane" :NewEnumerator1 "Bubble" :NewEnumerator2 "Cherry" :NewEnumerator3 "Blue Razz" :NewEnumerator4 "Lemon"))))

(fn ConstructionScript)