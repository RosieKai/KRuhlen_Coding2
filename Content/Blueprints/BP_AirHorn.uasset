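; BP_AirHorn is an air horn item that can be picked up, dropped and used to play horn sounds.
; Pickup snaps it to the BPI_ItemSocket socket on the given skeletal mesh and disables collision, with debug prints around the attach.
; Drop detaches it, moves it to the target location and restores collision.
; Primary and secondary use play normal and reversed horn sounds as non-spatialized 2D audio.
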(event EventPickup
  (params (skeletalMesh :type Skeletal%20Mesh%20Component%20Object%20Reference))
  (Development|PrintString "Attempting Airhorn Pick Up")
  (Transformation|AttachComponentToComponent skeletalMesh "BPI_ItemSocket" "SnapToTarget" "SnapToTarget" "KeepRelative" true)
  (Collision|SetCollisionEnabled (Variables|Default|GetCollision) "NoCollision")
  (Development|PrintString "PicAttempted"))

(event EventDrop
  (params (targetLocation :type Vector :default "0, 0, 0"))
  (Transformation|DetachFromActor "KeepRelative" "KeepRelative" "KeepRelative")
  (Transformation|SetActorLocation targetLocation false false)
  (Collision|SetCollisionEnabled (Variables|Default|GetCollision) "QueryAndPhysics"))

(event EventUsePrimary
  (Audio|PlaySound2D "/Game/Audio/Air_Horn_Normal.Air_Horn_Normal" 1.0 1.0 0.0 0 0))

(event EventUseSecondary
  (Audio|PlaySound2D "/Game/Audio/Air_Horn_Reverse.Air_Horn_Reverse" 1.0 1.0 0.0 0 0))

(fn ConstructionScript)