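; BP_Loops_Listss is a test Blueprint that demonstrates loop types and array iteration through on-screen prints.
; BeginPlay runs only a For Loop, printing indices in colors taken from an array.
; An uncalled DelayLoop event re-triggers itself through Delay and DoN, also starting a While countdown on LocCount.
; An uncalled ForEach event prints each color element in its own color.
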(event Custom|Delay%20Loop
  (Development|PrintText (Utilities|Text|FormatText "This has run {count} times" (stale _counter)))
  (Utilities|FlowControl|Delay 1.0)
  (bind _counter (Utilities|FlowControl|DoN 20)
    (:Exit
      (CallFunction|StartWhileLoop)
      (CallFunction|DelayLoop))))

(event Custom|StartForLoop
  (bind _array (Utilities|Array|MakeArray "(R=0.487212,G=1.000000,B=0.604154,A=1.000000)" "(R=1.000000,G=0.101062,B=0.985561,A=1.000000)" "(R=0.427348,G=0.118378,B=1.000000,A=1.000000)" "(R=0.200239,G=0.622769,B=1.000000,A=1.000000)" "(R=1.000000,G=0.891408,B=0.114135,A=1.000000)" "(R=1.000000,G=0.524568,B=0.408363,A=1.000000)"))
  (for _index (range 0 (- (Utilities|Array|Length _array) 1) 2)
    (Development|PrintText (Utilities|Text|FormatText "This is index {index}" _index) true true (Utilities|Array|Get(acopy) _array _index))))

(event Custom|StartWhileLoop
  (CallFunction|WhileTest))

(event Custom|StartForEachLoop
  (for (_array_element _array_index) (Utilities|Array|MakeArray "(R=0.487212,G=1.000000,B=0.604154,A=1.000000)" "(R=1.000000,G=0.101062,B=0.985561,A=1.000000)" "(R=0.427348,G=0.118378,B=1.000000,A=1.000000)" "(R=0.200239,G=0.622769,B=1.000000,A=1.000000)" "(R=1.000000,G=0.891408,B=0.114135,A=1.000000)" "(R=1.000000,G=0.524568,B=0.408363,A=1.000000)")
    (Development|PrintText (Utilities|Text|FormatText "Element {index} is pretty" _array_index) true true _array_element)))

(event EventBeginPlay
  (Development|PrintString "LL BP Exists")
  (CallFunction|StartforLoop))

(fn ConstructionScript)

(fn WhileTest
  (bind _loccount (LocalVariables|GetlocCount))
  (while (> _loccount 0)
    (Development|PrintText (Utilities|Text|FormatText "There are {uses} more uses in this loop" 0) true true "(R=0.203123,G=1.000000,B=0.119805,A=1.000000)")
    (Math|Integer|DecrementInt _loccount))
  (Development|PrintText (Utilities|Text|FormatText "You've run out of uses") true true "(R=1.000000,G=0.127484,B=0.179242,A=1.000000)"))