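; Crow alarm that gives away the player character when it enters the crow's sphere trigger.
; BeginPlay caches the crow's location, which the overlap uses to emit a pawn noise and play a placeholder sine ping slightly offset along X.
; The noise passes an explicit position instead of the noise maker's location, and debug text prints the crow's coordinates.
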(event OnComponentBeginOverlap(Sphere)
  (params (OverlappedComponent :type Primitive%20Component%20Object%20Reference) (OtherActor :type Actor%20Object%20Reference) (OtherComp :type Primitive%20Component%20Object%20Reference) (OtherBodyIndex :type Integer) (bFromSweep :type Boolean) (SweepResult :type Hit%20Result%20Structure%20%28by%20ref%29))
  (bind _self self)
  (bind _crocation (Variables|Default|GetCrocation))
  (bind _crocation_2 (Variables|Default|GetCrocation))
  (bind _returnvalue (+ (.x _crocation) 5e+01))
  (Utilities|Casting|CastToBP_ThirdPersonCharacter OtherActor)
  (Class|Pawn|PawnMakeNoise _self 2.0 (Math|Vector|MakeVector _returnvalue (.y _crocation) (.z _crocation)) false _self)
  (Audio|PlaySoundatLocation "/Engine/EngineSounds/1kSineTonePing.1kSineTonePing" (Math|Vector|MakeVector _returnvalue (.y _crocation) (.z _crocation)) "0, 0, 0" 1.0 1.0 0.0 0 0 0 0)
  (Development|PrintText (Utilities|Text|FormatText "Crow: X: {X} Y: {Y} Z: {Z}" (.x _crocation_2) (.y _crocation_2) (.z _crocation_2)) true true "(R=0.194874,G=0.000000,B=1.000000,A=1.000000)" 5.0))

(event EventBeginPlay
  (Variables|Default|SetCrocation (Transformation|GetActorLocation)))

(event Collision|EventActorBeginOverlap
  (params (OtherActor :type Actor%20Object%20Reference)))

(event EventTick
  (params (DeltaSeconds :type Float%20%28single-precision%29)))

(fn ConstructionScript)