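; Base enemy character providing patrol, melee, aggro and health behavior, with state variables for sight and hearing responses.
; It picks a random patrol route if unset and ping-pongs along its spline points.
; Attacks sphere-trace on a montage notify to hurt the player, while material swaps show aggro or curiosity.
; Health changes switch health-seeking enemies to Healing at half health; death ragdolls, spawns a lightning rod for cowards, then destroys the actor.
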(event Custom|Attack
  (bind _returnvalue (Transformation|GetActorLocation))
  (Audio|PlaySoundatLocation "/Game/Audio/SFX/Attack2.Attack2" (Transformation|GetActorLocation) "0, 0, 0" 1.0 1.0 0.0 0 0 0 0)
  (Animation|Montage|PlayMontage (Variables|Character|GetMesh) "/Game/CloseCombatAnimSet/Animations/InPlace/Attacks/NinjaLeftHook_Montage.NinjaLeftHook_Montage"
    (:OnCompleted
      (Default|CallAttackFinished :!label _label))
    (:OnInterrupted
      (goto _label))
    (:OnNotifyBegin
      (bind (_outhit _returnvalue_2) (Collision|SphereTraceByChannel _returnvalue (+ _returnvalue (* (Transformation|GetActorForwardVector) 1e+02)) 5e+01 "TraceTypeQuery2" false 0 "ForDuration"))
      (if _returnvalue_2
        (bind _asbp_third_person_character (Utilities|Casting|CastToBP_ThirdPersonCharacter (.HitActor (Collision|BreakHitResult _outhit))))
        (Default|ChangeHealth _asbp_third_person_character (Variables|Default|GetAttack%20Damage))
        (Default|HurtSound _asbp_third_person_character)))))

(event Custom|GetAggro
  (Rendering|Material|SetMaterial (Variables|Character|GetMesh) 0 "/AnimationSharing/AnimSharingRed.AnimSharingRed")
  (Variables|Default|SetAggroed true))

(event Custom|LoseAggro
  (Rendering|Material|SetMaterial (Variables|Character|GetMesh) 0 (Variables|Default|GetOriginalMaterial))
  (Variables|Default|SetAggroed false))

(event Custom|SetWalkSpeed
  (params (Speed :type Float%20%28double-precision%29))
  (Variables|/Script/Engine.CharacterMovementComponent|SetMaxWalkSpeed (Variables|Character|GetCharacterMovement) Speed))

(event Custom|Set%20Curious%20Color
  (Rendering|Material|SetMaterial (Variables|Character|GetMesh) 0 "/AnimationSharing/AnimSharingGreen.AnimSharingGreen"))

(event Custom|Ragdoll
  (params (Origin :type Vector))
  (bind _mesh (Variables|Character|GetMesh))
  (Physics|SetSimulatePhysics _mesh true)
  (Physics|AddRadialImpulse _mesh (+ Origin "0.000000,0.000000,-50.000000") 3e+02 5e+03 "RIF_Constant" true)
  (Pawn|Components|CharacterMovement|DisableMovement (Variables|Character|GetCharacterMovement))
  (if (Variables|Default|GetCoward)
    (Game|SpawnActorfromClass "/Game/Blueprints/BP_LightningRod.BP_LightningRod_C" (Math|Transform|MakeTransform Origin "0, 0, 0" "1.000000,1.000000,1.000000") "Undefined" "MultiplyWithRoot" 0 0))
  (Utilities|FlowControl|Delay 1.0)
  (Actor|DestroyActor))

(event Custom|Set%20Healed%20State
  (Variables|BehaviorStates|SetCurrentSeeState (Variables|BehaviorStates|GetHealedSeeState))
  (Variables|BehaviorStates|SetCurrentHearState (Variables|BehaviorStates|GetHealedHearState)))

(event EventBeginPlay
  (Utilities|IsValid (Variables|PatrolRoute|GetPatrolRoute)
    (:Is%20Valid
      _)
    (:Is%20Not%20Valid
      (bind _outactors (Actor|GetAllActorsOfClass "/Game/AI_Blueprints/BP_PatrolRoute.BP_PatrolRoute_C"))
      (Variables|PatrolRoute|SetPatrolRoute (.OutItem (Utilities|Array|Random _outactors)))))
  (Variables|Default|SetOriginalMaterial (Rendering|Material|GetMaterial (Variables|Character|GetMesh) 0))
  (Variables|Default|SetMaxHealth (Variables|Default|GetHealth)))

(event Game|Damage|EventPointDamage
  (params (Damage :type Float%20%28single-precision%29) (DamageType :type Damage%20Type%20Object%20Reference) (HitLocation :type Vector :default "0, 0, 0") (HitNormal :type Vector :default "0, 0, 0") (HitComponent :type Primitive%20Component%20Object%20Reference) (BoneName :type Name :default "None") (ShotFromDirection :type Vector :default "0, 0, 0") (InstigatedBy :type Controller%20Object%20Reference) (DamageCauser :type Actor%20Object%20Reference) (HitInfo :type Hit%20Result%20Structure%20%28by%20ref%29))
  (Development|PrintText (Utilities|Text|FormatText "{Instigator} hit me for {dmg} damage!" InstigatedBy Damage))
  (bind _output_get (Variables|Default|SetHealth (- (Variables|Default|GetHealth) Damage)))
  (CallFunction|CheckHealth)
  (if (<= _output_get 0.0)
    (Audio|PlaySoundatLocation "/Game/Audio/SFX/Death1.Death1" HitLocation "0, 0, 0" 1.0 1.0 0.0 0 0 0 0)
    (CallFunction|Ragdoll ShotFromDirection)
    (Development|PrintString "I HAVE PERISHED")
    (else
      (Audio|PlaySoundatLocation "/Game/Audio/SFX/Hit1.Hit1" HitLocation "0, 0, 0" 1.0 1.0 0.0 0 0 0 0))))

(event EventHeal
  (params (HealthAmount :type Float%20%28double-precision%29))
  (Variables|Default|SetHealth (+ HealthAmount (Variables|Default|GetHealth)))
  (bind _currenthealth (CallFunction|CheckHealth))
  (switch Utilities|FlowControl|Switch|SwitchonE_AI_State (Variables|BehaviorStates|GetCurrentSeeState)
    (:NewEnumerator0
      (Development|PrintString "waiting"))
    (:NewEnumerator1
      (Development|PrintString "patroling"))
    (:NewEnumerator2
      (Development|PrintText (Utilities|Text|FormatText "Current Health: {Health} Current State: Attacking" _currenthealth) true true "(R=0.000000,G=0.404547,B=1.000000,A=1.000000)" 5.0))
    (:NewEnumerator3
      (Development|PrintString "investigatng"))
    (:NewEnumerator4
      (Development|PrintString "retreating"))
    (:NewEnumerator5
      (Development|PrintString "healing"))))

(event Game|Damage|EventRadialDamage
  (params (DamageReceived :type Float%20%28single-precision%29) (DamageType :type Damage%20Type%20Object%20Reference) (Origin :type Vector :default "0, 0, 0") (HitInfo :type Hit%20Result%20Structure%20%28by%20ref%29) (InstigatedBy :type Controller%20Object%20Reference) (DamageCauser :type Actor%20Object%20Reference))
  (Development|PrintText (Utilities|Text|FormatText "{Instigator} hit me for {dmg} damage!" InstigatedBy DamageReceived))
  (bind _output_get (Variables|Default|SetHealth (- (Variables|Default|GetHealth) DamageReceived)))
  (CallFunction|CheckHealth)
  (if (<= _output_get 0.0)
    (CallFunction|Ragdoll Origin)
    (Development|PrintString "I HAVE PERISHED")))

(fn ConstructionScript)

(fn GetPatrolPoint
  (bind _output_get (Variables|PatrolRoute|SetPatrolIndex (+ (Variables|PatrolRoute|GetPatrolIndex) (Variables|PatrolRoute|GetDirection))))
  (Development|PrintText (Utilities|Text|FormatText "Going to point {point}" _output_get))
  (if (or (>= (+ (Variables|PatrolRoute|GetPatrolIndex) 1) (Spline|GetNumberOfSplinePoints (Variables|/Game/AI_Blueprints/BP_PatrolRoute.BP_PatrolRoute_C|GetSpline (Variables|PatrolRoute|GetPatrolRoute)))) (<= (Variables|PatrolRoute|GetPatrolIndex) 0))
    (Variables|PatrolRoute|SetDirection (* (Variables|PatrolRoute|GetDirection) -1)))
  (return (Spline|GetLocationatSplinePoint (Variables|/Game/AI_Blueprints/BP_PatrolRoute.BP_PatrolRoute_C|GetSpline (Variables|PatrolRoute|GetPatrolRoute)) (Variables|PatrolRoute|GetPatrolIndex) "World")))

(fn GetIdealRange
  (return (Variables|Default|GetAttack%20Range) (Variables|Default|GetStrafe%20Range)))

(fn CheckHealth
  (bind _takeshealth (Variables|Default|GetTakesHealth))
  (bind _maxhealth (Variables|Default|GetMaxHealth))
  (bind _health (Variables|Default|GetHealth))
  (bind _returnvalue (* _maxhealth 0.5))
  (bind _returnvalue_2 (<= _health _returnvalue))
  (bind _returnvalue_3 (and _returnvalue_2 _takeshealth))
  (Development|PrintString (Utilities|String|ToString(Boolean) _returnvalue_3))
  (if _returnvalue_3
    (Variables|BehaviorStates|SetCurrentSeeState "NewEnumerator5")
    (Variables|BehaviorStates|SetCurrentHearState "NewEnumerator5")
    (else
      (Variables|BehaviorStates|SetCurrentSeeState (Variables|BehaviorStates|GetHealedSeeState))
      (Variables|BehaviorStates|SetCurrentHearState (Variables|BehaviorStates|GetHealedHearState))))
  (return _health _maxhealth _returnvalue_3))