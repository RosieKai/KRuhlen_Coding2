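; BP_Decoy is a deployable noise decoy that emits an AI-audible noise after a random delay of a few seconds.
; Deploy starts the BeepBeep loop, which flip-flops the mesh material at a shrinking, clamped interval while Blink is set.
; When the timer clears Blink, the decoy makes a loud pawn noise at its location, briefly plays audio and destroys itself.
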(event Custom|BeepBeep
  (bind _audio (Variables|Default|GetAudio))
  (bind _staticmesh (Variables|Default|GetStaticMesh))
  (if (Variables|Default|GetBlink) :!label _label
    (Utilities|FlowControl|FlipFlop
      (:A
        (Rendering|Material|SetMaterial _staticmesh 0 "/Game/Materials/MI_E_Yellow.MI_E_Yellow"))
      (:B
        (Rendering|Material|SetMaterial _staticmesh 0 "/Game/Fab/Pato_Fallguys/pato_fallguys/Materials/CUERPAZO.CUERPAZO")))
    (Utilities|FlowControl|Delay (Variables|Default|GetblinkTime))
    (Variables|Default|SetblinkTime (Math|Float|Clamp(Float) (/ (Variables|Default|GetblinkTime) 1.25) 0.1))
    (goto _label)
    (else
      (Rendering|Material|SetMaterial _staticmesh 0 "/Game/Materials/MI_E_Yellow.MI_E_Yellow")
      (Class|Pawn|PawnMakeNoise 4.0 (Transformation|GetActorLocation) false 0)
      (Audio|Components|Audio|Play _audio 0.0)
      (Utilities|FlowControl|Delay 2.0)
      (Audio|Components|Audio|Stop _audio)
      (Actor|DestroyActor))))

(event Custom|Deploy
  (CallFunction|BeepBeep)
  (Utilities|FlowControl|Delay (Math|Random|RandomFloatinRange 3.0 7.0))
  (Variables|Default|SetBlink false))

(fn ConstructionScript)